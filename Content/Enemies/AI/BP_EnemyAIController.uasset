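; BP_EnemyAIController is an AI controller for BP_Enemy pawns.
; On BeginPlay it casts and caches the BP_BardPlayer character and its controlled enemy.
; An unconnected AIMoveTo chain would move the enemy to the player and set its CanAttack flag on success or failure, but it never runs.
; Tick is empty, so the controller currently drives no movement or attack logic.
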(event `self.ReceiveBeginPlay`
  (bind _asbp_bard_player (cast `/Game/BardCharacter/BP_BardPlayer` (`GameplayStatics.GetPlayerCharacter` 0)))
  (set `self.As BP Bard Player` _asbp_bard_player)
  (bind _asbp_enemy (cast `/Game/Enemies/BP_Enemy` (`self.K2_GetPawn`)))
  (set `self.As BP Enemy` _asbp_enemy))

(event `self.ReceiveTick`
  (params (DeltaSeconds :type "Float (single-precision)")))

(fn `UserConstructionScript`)